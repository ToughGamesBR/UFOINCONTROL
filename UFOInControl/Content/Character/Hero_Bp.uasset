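; Player hero Blueprint with camera control, thruster-gated movement and four selectable energy-draining tools: hook, radio, claw and USB.
; The thruster toggle and AtivarArma adjust Consumo, while AtivarArma also sets the active tool's range.
; Tick feeds Consumo through a Delay as self-damage, lowering clamped Energia and restarting the level at zero.
; Left click line-traces WorldDynamic objects within range and sends the hit actor that tool's interaction message.
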(event Game|Damage|EventAnyDamage
  (params (Damage :type Float%20%28single-precision%29) (DamageType :type Damage%20Type%20Object%20Reference) (InstigatedBy :type Controller%20Object%20Reference) (DamageCauser :type Actor%20Object%20Reference))
  ;[1 1 1] Aplica Dano
  (bind _qtdenergia (CallFunction|AddEnergia (* Damage -1.0)))
  (if (<= _qtdenergia 0.0)
    (Utilities|FlowControl|Delay 1.0)
    (Development|ExecuteConsoleCommand "restartLevel" 0)))

(event EventTick
  (params (DeltaSeconds :type Float%20%28single-precision%29))
  ;[1 1 1] Consome Energia
  (Rendering|Components|TextRender|SetText (Variables|Default|GetTextoEnergia) (Utilities|Text|ToText(Float) (Variables|Default|GetEnergia) "HalfToEven"))
  (Utilities|FlowControl|Delay 1.0)
  (Game|Damage|ApplyDamage self (Variables|Default|GetConsumo) 0 0)
  (Development|PrintString (Utilities|String|ToString(Text) (Variables|Default|GetArmaAtiva))))

(event Input|ActionEvents|InputActionSelectArmPropulsor
  (params (Key :type Key%20Structure))
  ;[1 1 1] Propulsor
  (:Pressed
    (Utilities|FlowControl|FlipFlop
      (:A
        (Variables|Default|SetAtivouPropulsor true)
        (CallFunction|AddConsumo 0.002))
      (:B
        (Variables|Default|SetAtivouPropulsor false)
        (CallFunction|AddConsumo -0.02)))))

(event Input|ActionEvents|InputActionSelectArmRadio
  (params (Key :type Key%20Structure))
  ;[1 1 1] Radio
  (:Pressed
    (CallFunction|AtivarArma "radio" 0.003 5e+02)))

(event Input|ActionEvents|InputActionSelectArmGancho
  (params (Key :type Key%20Structure))
  ;[1 1 1] Gancho
  (:Pressed
    (CallFunction|AtivarArma "gancho" 0.004 5e+02)))

(event Input|ActionEvents|InputActionSelectArmGarra
  (params (Key :type Key%20Structure))
  ;[1 1 1] Garra
  (:Pressed
    (CallFunction|AtivarArma "garra" 0.002 5e+01)))

(event Input|ActionEvents|InputActionSelectArmUSB
  (params (Key :type Key%20Structure))
  ;[1 1 1] USB
  (:Pressed
    (CallFunction|AtivarArma "usb" 0.001 5e+01)))

(event Input|AxisEvents|InputAxisMoveForward
  (params (AxisValue :type Float%20%28single-precision%29))
  ;[1 1 1] Movimento
  (if (Variables|Default|GetAtivouPropulsor)
    (Pawn|Input|AddMovementInput (Math|Vector|GetForwardVector (Math|Rotator|MakeRotator 0.0 0.0 (.yaw (Pawn|GetControlRotation :!class /Script/Engine.Pawn)))) AxisValue false)))

(event Input|AxisEvents|InputAxisMoveSides
  (params (AxisValue :type Float%20%28single-precision%29))
  ;[1 1 1] Movimento
  (if (Variables|Default|GetAtivouPropulsor)
    (Pawn|Input|AddMovementInput (Math|Vector|GetRightVector (Math|Rotator|MakeRotator 0.0 0.0 (.yaw (Pawn|GetControlRotation :!class /Script/Engine.Pawn)))) AxisValue false)))

(event Input|AxisEvents|InputAxisCameraTurn
  (params (AxisValue :type Float%20%28single-precision%29))
  ;[1 1 1] Camera
  (Pawn|Input|AddControllerYawInput AxisValue))

(event Input|AxisEvents|InputAxisCameraLookUp
  (params (AxisValue :type Float%20%28single-precision%29))
  ;[1 1 1] Camera
  (Pawn|Input|AddControllerPitchInput (* AxisValue -1.0)))

(event Input|MouseEvents|LeftMouseButton
  (params (Key :type Key%20Structure))
  (bind _returnvalue (Transformation|GetActorLocation))
  ;[1 1 1] Interação
  (:Pressed
    (bind (_outhit _returnvalue_2) (Collision|LineTraceForObjects _returnvalue (+ (* (Math|Vector|GetForwardVector (Pawn|GetControlRotation :!class /Script/Engine.Pawn)) (Variables|Default|GetArmaAlcance)) _returnvalue) (Utilities|Array|MakeArray "ObjectTypeQuery2") false 0 "None"))
    (if _returnvalue_2
      (switch string (Utilities|String|ToString(Text) (Variables|Default|GetArmaAtiva))
        (:gancho
          (Class|InteracaoArmas|InteragirGancho(Message) (.HitActor (Collision|BreakHitResult _outhit))))
        (:radio
          (Class|InteracaoArmas|InteragirRadio(Message) (.HitActor (Collision|BreakHitResult _outhit))))
        (:garra
          (Class|InteracaoArmas|InteragirGarra(Message) (.HitActor (Collision|BreakHitResult _outhit))))
        (:usb
          (Class|InteracaoArmas|InteragirUsb(Message) (.HitActor (Collision|BreakHitResult _outhit))))))))

(fn ConstructionScript)

(fn AddEnergia
  (params (addEnergia :type Float%20%28single-precision%29))
  (bind _output_get (Variables|Default|SetEnergia (Math|Float|Clamp(Float) (+ addEnergia (Variables|Default|GetEnergia)))))
  (return _output_get))

(fn AddConsumo
  (params (addConsumo :type Float%20%28single-precision%29))
  (bind _output_get (Variables|Default|SetConsumo (+ addConsumo (Variables|Default|GetConsumo))))
  (return _output_get))

(fn AtivarArma
  (params (ArmaAtivando :type Text) (ConsumoArmaAtivando :type Float%20%28single-precision%29) (AlcanceArmaAtivando :type Float%20%28single-precision%29))
  (if (Utilities|Enum|Equal(Enum) ArmaAtivando (Variables|Default|GetArmaAtiva))
    (CallFunction|AddConsumo (* (Variables|Default|GetConsumoArmaAtiva) -1.0))
    (Variables|Default|SetArmaAtiva "idle")
    (Variables|Default|SetConsumoArmaAtiva 0.0)
    (Variables|Default|SetArmaAlcance 0.0)
    (else
      (Variables|Default|SetArmaAtiva ArmaAtivando)
      (Variables|Default|SetArmaAlcance AlcanceArmaAtivando)
      (bind _output_get (Variables|Default|SetConsumoArmaAtiva ConsumoArmaAtivando))
      (CallFunction|AddConsumo _output_get))))